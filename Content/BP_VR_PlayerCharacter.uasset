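; VR player character that drives a Manny body from headset and motion controller transforms each tick.
; A child-actor keyboard types into the login widget's email and password fields, with login props hidden outside MainWorld levels.
; PlayerState data goes through a server event; its OnRep updates the name display and calls GameState's multicast, retrying by timer until the GameState cast succeeds.
; Right alternate grip toggles the phone settings widget; left-grip teleport is an empty WIP.
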(event `self.ReceiveBeginPlay`
  (bind _handmesh_right (`self.HandMesh-Right`))
  (`parent.ReceiveBeginPlay`)
  (bind _asue4_abp_manny (cast `/Game/Characters/Mannequin_UE4/Animations/UE4_ABP_Manny` (`SkeletalMeshComponent.GetAnimInstance` (`self.Mesh`))))
  (set `self.As UE4 ABP Manny` _asue4_abp_manny)
  (`SceneComponent.SetHiddenInGame` _handmesh_right true false)
  (`SceneComponent.SetHiddenInGame` (`self.HandMesh-Left`) true false)
  (`SceneComponent.SetVisibility` _handmesh_right false false)
  (`SceneComponent.SetVisibility` (`self.HandMesh-Left`) false false)
  (`|ExecutionSequence`
    (:`then_0`
      (bind _asbp_player_state (cast `/Game/Blueprints/PlayerState/BP_PlayerState` (`self.PlayerState`)))
      (bind _output_get (set `self.As BP Player State` _asbp_player_state))
      (add `/Game/Blueprints/PlayerState/BP_PlayerState.OnSendPlayerData` _output_get (delegate `OnSendPlayerData_Event`))
      (bind _asbp_game_instance (cast `/Game/Blueprints/Subsystem/BP_GameInstance` (`GameplayStatics.GetGameInstance`)))
      (set `self.As BP Game Instance` _asbp_game_instance))
    (:`then_1`
      (bind _returnvalue (`GameplayStatics.GetCurrentLevelName` true))
      (if (not (`KismetStringLibrary.Contains` _returnvalue "MainWorld"))
        (`SceneComponent.SetHiddenInGame` (`self.Iphone`) true false)
        (`SceneComponent.SetHiddenInGame` (`self.WidgetLogin`) true false)
        (`SceneComponent.SetHiddenInGame` (`self.Keyboard`) true false)))
    (:`then_2`
      (bind _askeyboard_test_actor (cast `/Game/VRE/Level/Keyboard/KeyboardTestActor` (`ChildActorComponent.ChildActor` (`self.Keyboard`))))
      (bind _output_get_2 (set `self.As Keyboard Test Actor` _askeyboard_test_actor))
      (add `/Game/VRE/Level/Keyboard/KeyboardTestActor.ClearText` _output_get_2 (delegate `ClearText_Event`))
      (add `/Game/VRE/Level/Keyboard/KeyboardTestActor.GetInputKeyboard` _output_get_2 (delegate `GetInputKeyboard_Event`))
      (bind _aswbp_login_fixed (cast `/Game/Blueprints/Widgets/WBP_Login_FIXED` (`WidgetComponent.GetUserWidgetObject` (`self.WidgetLogin`))))
      (set `self.As WBP Login FIXED` _aswbp_login_fixed))))

(event `OnSendPlayerData_Event`
  (params (PlayerData :type "/Game/Blueprints/Structure/S_PlayerData Structure"))
  (`self.Server_GetPlayerDataStruct` PlayerData)
  (`KismetSystemLibrary.PrintString` "3. PCharacter" true true (struct :`G` 0.66 :`B` 1.0 :`A` 1.0) 20.0))

(event `Server_GetPlayerDataStruct`
  (params (PlayerData :type "/Game/Blueprints/Structure/S_PlayerData Structure"))
  (set `self.PlayerData` PlayerData))

(event `self.ReceiveTick`
  (params (DeltaSeconds :type "Float (single-precision)"))
  (bind _as_ue4_abp_manny (`self.As UE4 ABP Manny`))
  (`parent.ReceiveTick` DeltaSeconds)
  (`/Engine/EditorBlueprintResources/StandardMacros.IsValid` _as_ue4_abp_manny
    (:`Is Valid`
      (set `/Game/Characters/Mannequin_UE4/Animations/UE4_ABP_Manny.HeadTransform` (`SceneComponent.K2_GetComponentToWorld` (`self.VRReplicatedCamera`)) _as_ue4_abp_manny)
      (set `/Game/Characters/Mannequin_UE4/Animations/UE4_ABP_Manny.LeftTransform` (`SceneComponent.K2_GetComponentToWorld` (`self.LeftMotionController`)) _as_ue4_abp_manny)
      (set `/Game/Characters/Mannequin_UE4/Animations/UE4_ABP_Manny.RightTransform` (`SceneComponent.K2_GetComponentToWorld` (`self.RightMotionController`)) _as_ue4_abp_manny))))

(event `EnhancedInput|/Game/VRE/Input/Actions/AlternateGripRight`
  (params (ActionValue :type Boolean) (ElapsedSeconds :type "Float (double-precision)") (TriggeredSeconds :type "Float (double-precision)") (InputAction :type "InputAction Object Reference" :default "/Game/VRE/Input/Actions/AlternateGripRight.AlternateGripRight"))
  (bind _iphone (`self.Iphone`))
  (:`Started`
    (`/Engine/EditorBlueprintResources/StandardMacros.FlipFlop`
      (:`A`
        (`SceneComponent.SetHiddenInGame` _iphone false false)
        (`SceneComponent.SetHiddenInGame` (`self.WidgetSettings`) false false))
      (:`B`
        (`SceneComponent.SetHiddenInGame` _iphone true false)
        (`SceneComponent.SetHiddenInGame` (`self.WidgetSettings`) true false)))))

(event `ClearText_Event`
  (bind _as_wbp_login_fixed (`self.As WBP Login FIXED`))
  (switch `/Game/Blueprints/Enum/EEditableText` (`/Game/Blueprints/Widgets/WBP_Login_FIXED.EditableText` _as_wbp_login_fixed)
    (:`NewEnumerator0`
      (`EditableText.SetText` (`/Game/Blueprints/Widgets/WBP_Login_FIXED.InputEmail` _as_wbp_login_fixed) ""))
    (:`NewEnumerator1`
      (`EditableText.SetText` (`/Game/Blueprints/Widgets/WBP_Login_FIXED.InputPassword` _as_wbp_login_fixed) ""))))

(event `GetInputKeyboard_Event`
  (params (InText :type Text))
  (bind _as_wbp_login_fixed (`self.As WBP Login FIXED`))
  (bind _inputemail (`/Game/Blueprints/Widgets/WBP_Login_FIXED.InputEmail` _as_wbp_login_fixed))
  (bind _inputpassword (`/Game/Blueprints/Widgets/WBP_Login_FIXED.InputPassword` _as_wbp_login_fixed))
  (set `self.DisplayText` InText)
  (switch `/Game/Blueprints/Enum/EEditableText` (`/Game/Blueprints/Widgets/WBP_Login_FIXED.EditableText` _as_wbp_login_fixed)
    (:`NewEnumerator0`
      (`EditableText.SetText` _inputemail (`|FormatText` "{original}{addedText}" (`EditableText.Text` _inputemail) (`self.DisplayText`))))
    (:`NewEnumerator1`
      (`EditableText.SetText` _inputpassword (`|FormatText` "{original}{addedText}" (`EditableText.Text` _inputpassword) (`self.DisplayText`))))))

(event `EnhancedInput|/Game/VRE/Input/Actions/AlternateGripLeft`
  (params (ActionValue :type Boolean) (ElapsedSeconds :type "Float (double-precision)") (TriggeredSeconds :type "Float (double-precision)") (InputAction :type "InputAction Object Reference" :default "/Game/VRE/Input/Actions/AlternateGripLeft.AlternateGripLeft")))

(fn `OnRep_PlayerData`
  (bind (_playerstate _playername) (break `/Game/Blueprints/Structure/S_PlayerData` (`self.PlayerData`)))
  (`TextRenderComponent.K2_SetText` (`self.PlayerNameDisplay`) (`KismetTextLibrary.Conv_StringToText` _playername))
  (`KismetSystemLibrary.PrintString` (`KismetStringLibrary.Concat_StrStr` "3. " _playername) true true (struct :`G` 0.66 :`B` 1.0 :`A` 1.0) 50.0)
  (bind _asbp_game_state (cast `/Game/Blueprints/GameState/BP_GameState` (`GameplayStatics.GetGameState`))
    (:`then`
      (`/Game/Blueprints/GameState/BP_GameState.Multicast_RetrievePlayerData` _asbp_game_state (`self.PlayerData`)))
    (:`CastFailed`
      (`KismetSystemLibrary.K2_SetTimer` null "OnRep_PlayerData" 0.1))))

(fn `UserConstructionScript`
  (`parent.UserConstructionScript`))